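; Speaker actor built from cabinet, accent, screen and driver meshes that serves as a clickable, hoverable model for a speaker controller Blueprint.
; InitialiseSpeakerBP stores the controller reference, and mouse events on each part forward clicks and hint requests to it by part group.
; A SetCoverActive flag controls whether the front frame and screen are hidden and made non-interactive.
; Getter functions expose each group's mesh components.
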(event `self.ReceiveBeginPlay`
  (bind _frame (`self.Frame`))
  (bind _screen (`self.Screen`))
  ;[1 1 1] Hide screen and frame if cover inactive checked
  (if (not (`self.SetCoverActive`))
    (`SceneComponent.SetVisibility` _frame false false)
    (`PrimitiveComponent.SetCollisionEnabled` _frame "NoCollision")
    (`SceneComponent.SetVisibility` _screen false false)
    (`PrimitiveComponent.SetCollisionEnabled` _screen "NoCollision")))

(event `self.Foot_BL.OnClicked`
  (params (TouchedComponent :type "PrimitiveComponent Object Reference") (ButtonPressed :type "Key Structure"))
  ;[1 1 1] Accents Clicked
  (`/Game/Spkrs/BP/SpeakerController_BP.AccentClicked` (`self.Speaker Controller BP ref`) :!label _label))

(event `self.Foot_BR.OnClicked`
  (params (TouchedComponent :type "PrimitiveComponent Object Reference") (ButtonPressed :type "Key Structure"))
  ;[1 1 1] Accents Clicked
  (goto _label))

(event `self.Foot_FL.OnClicked`
  (params (TouchedComponent :type "PrimitiveComponent Object Reference") (ButtonPressed :type "Key Structure"))
  ;[1 1 1] Accents Clicked
  (goto _label))

(event `self.Foot_FR.OnClicked`
  (params (TouchedComponent :type "PrimitiveComponent Object Reference") (ButtonPressed :type "Key Structure"))
  ;[1 1 1] Accents Clicked
  (goto _label))

(event `self.AccentPlate.OnClicked`
  (params (TouchedComponent :type "PrimitiveComponent Object Reference") (ButtonPressed :type "Key Structure"))
  ;[1 1 1] Accents Clicked
  (goto _label))

(event `self.Frame.OnClicked`
  (params (TouchedComponent :type "PrimitiveComponent Object Reference") (ButtonPressed :type "Key Structure"))
  ;[1 1 1] Accents Clicked
  (goto _label))

(event `self.HornTweeter.OnClicked`
  (params (TouchedComponent :type "PrimitiveComponent Object Reference") (ButtonPressed :type "Key Structure"))
  ;[1 1 1] Speakers  Clicked
  (`/Game/Spkrs/BP/SpeakerController_BP.SpeakerClicked` (`self.Speaker Controller BP ref`) :!label _label_2))

(event `self.Woofers.OnClicked`
  (params (TouchedComponent :type "PrimitiveComponent Object Reference") (ButtonPressed :type "Key Structure"))
  ;[1 1 1] Speakers  Clicked
  (goto _label_2))

(event `self.Screen.OnClicked`
  (params (TouchedComponent :type "PrimitiveComponent Object Reference") (ButtonPressed :type "Key Structure"))
  ;[1 1 1] Screen  Clicked
  (`/Game/Spkrs/BP/SpeakerController_BP.ScreenClicked` (`self.Speaker Controller BP ref`)))

(event `self.Cabinette.OnClicked`
  (params (TouchedComponent :type "PrimitiveComponent Object Reference") (ButtonPressed :type "Key Structure"))
  ;[1 1 1] Cabinet  Clicked
  (`/Game/Spkrs/BP/SpeakerController_BP.CabinetClicked` (`self.Speaker Controller BP ref`)))

(event `self.Cabinette.OnBeginCursorOver`
  (params (TouchedComponent :type "PrimitiveComponent Object Reference"))
  ;[1 1 1] Display controller hints on mouseover
  (`/Game/Spkrs/BP/SpeakerController_BP.DisplayCabinetHint` (`self.Speaker Controller BP ref`)))

(event `self.AccentPlate.OnBeginCursorOver`
  (params (TouchedComponent :type "PrimitiveComponent Object Reference"))
  ;[1 1 1] Display controller hints on mouseover
  (`/Game/Spkrs/BP/SpeakerController_BP.DisplayAccentHint` (`self.Speaker Controller BP ref`) :!label _label_3))

(event `self.Frame.OnBeginCursorOver`
  (params (TouchedComponent :type "PrimitiveComponent Object Reference"))
  ;[1 1 1] Display controller hints on mouseover
  (goto _label_3))

(event `self.Foot_BL.OnBeginCursorOver`
  (params (TouchedComponent :type "PrimitiveComponent Object Reference"))
  ;[1 1 1] Display controller hints on mouseover
  (goto _label_3))

(event `self.Foot_BR.OnBeginCursorOver`
  (params (TouchedComponent :type "PrimitiveComponent Object Reference"))
  ;[1 1 1] Display controller hints on mouseover
  (goto _label_3))

(event `self.Foot_FL.OnBeginCursorOver`
  (params (TouchedComponent :type "PrimitiveComponent Object Reference"))
  ;[1 1 1] Display controller hints on mouseover
  (goto _label_3))

(event `self.Foot_FR.OnBeginCursorOver`
  (params (TouchedComponent :type "PrimitiveComponent Object Reference"))
  ;[1 1 1] Display controller hints on mouseover
  (goto _label_3))

(event `self.Screen.OnBeginCursorOver`
  (params (TouchedComponent :type "PrimitiveComponent Object Reference"))
  ;[1 1 1] Display controller hints on mouseover
  (`/Game/Spkrs/BP/SpeakerController_BP.DisplayScreenHint` (`self.Speaker Controller BP ref`)))

(event `self.Woofers.OnBeginCursorOver`
  (params (TouchedComponent :type "PrimitiveComponent Object Reference"))
  ;[1 1 1] Display controller hints on mouseover
  (`/Game/Spkrs/BP/SpeakerController_BP.DisplaySpeakerHint` (`self.Speaker Controller BP ref`) :!label _label_4))

(event `self.HornTweeter.OnBeginCursorOver`
  (params (TouchedComponent :type "PrimitiveComponent Object Reference"))
  ;[1 1 1] Display controller hints on mouseover
  (goto _label_4))

(event `self.Cabinette.OnEndCursorOver`
  (params (TouchedComponent :type "PrimitiveComponent Object Reference"))
  ;[1 1 1] Display general hint for controlls when not moused over
  (`/Game/Spkrs/BP/SpeakerController_BP.DisplayGeneralHint` (`self.Speaker Controller BP ref`) :!label _label_5))

(event `self.Foot_BL.OnEndCursorOver`
  (params (TouchedComponent :type "PrimitiveComponent Object Reference"))
  ;[1 1 1] Display general hint for controlls when not moused over
  (goto _label_5))

(event `self.Foot_BR.OnEndCursorOver`
  (params (TouchedComponent :type "PrimitiveComponent Object Reference"))
  ;[1 1 1] Display general hint for controlls when not moused over
  (goto _label_5))

(event `self.Foot_FL.OnEndCursorOver`
  (params (TouchedComponent :type "PrimitiveComponent Object Reference"))
  ;[1 1 1] Display general hint for controlls when not moused over
  (goto _label_5))

(event `self.Foot_FR.OnEndCursorOver`
  (params (TouchedComponent :type "PrimitiveComponent Object Reference"))
  ;[1 1 1] Display general hint for controlls when not moused over
  (goto _label_5))

(event `self.Frame.OnEndCursorOver`
  (params (TouchedComponent :type "PrimitiveComponent Object Reference"))
  ;[1 1 1] Display general hint for controlls when not moused over
  (goto _label_5))

(fn `GetAccentComponents`
  (returns (FootMeshes :type "Array of StaticMeshComponent Object Reference") (AccentMeshes :type "Array of StaticMeshComponent Object Reference"))
  (return (`|MakeArray` (`self.Foot_BL`) (`self.Foot_BR`) (`self.Foot_FL`) (`self.Foot_FR`)) (`|MakeArray` (`self.AccentPlate`) (`self.Frame`))))

(fn `GetCabinetComponent`
  (returns (CabinetMesh :type "StaticMeshComponent Object Reference"))
  (return (`self.Cabinette`)))

(fn `GetScreenComponent`
  (returns (ScreenMesh :type "StaticMeshComponent Object Reference"))
  (return (`self.Screen`)))

(fn `GetSpeakerComponents`
  (returns (TweeterMesh :type "StaticMeshComponent Object Reference") (SpeakerMesh :type "StaticMeshComponent Object Reference"))
  (return (`self.HornTweeter`) (`self.Woofers`)))

(fn `InitialiseSpeakerBP`
  (params (`Speaker Controller BP` :type "/Game/Spkrs/BP/SpeakerController_BP Object Reference"))
  (`|ExecutionSequence`
    (:`then_0`
      (set `self.Speaker Controller BP ref` `Speaker Controller BP`))
    (:`then_1`
      ;[1 1 1] Set Cover Active
      (if (`self.SetCoverActive`)
        ;;[0 1 0.1458] Cover Active
        (`SceneComponent.SetVisibility` (`self.Frame`) true false)
        (`SceneComponent.SetVisibility` (`self.Screen`) true false)
        (else
          ;;[1 0 0.008924] Cover Not Active
          (`SceneComponent.SetVisibility` (`self.Frame`) false false)
          (`SceneComponent.SetVisibility` (`self.Screen`) false false)
          (`PrimitiveComponent.SetCollisionResponseToAllChannels` (`self.Frame`) "ECR_Ignore")
          (`PrimitiveComponent.SetCollisionResponseToAllChannels` (`self.Screen`) "ECR_Ignore"))))))

(fn `UserConstructionScript`)