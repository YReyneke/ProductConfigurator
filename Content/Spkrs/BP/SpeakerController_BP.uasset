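; Controller for a speaker product configurator that cycles cabinet, driver, accent and screen finishes across every speaker in the scene.
; Each click function advances a wrapping index and applies materials or a colour parameter via the speakers' component getters.
; Matching data table rows supply descriptions and prices, pushed to the HUD with a GBP total.
; It also sets hint text, room background colour, and music track and volume.
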(fn `AccentClicked`
  (bind _output_get (set `self.AccentIndex` (mod (+ (`self.AccentIndex`) 1) (`self.AccentIndexMax`))))
  (switch `int` _output_get
    (:`0`
      (`self.SetAccentMaterials` "/Game/Spkrs/m/BlkGld_Ft.BlkGld_Ft" "/Game/Spkrs/m/BlkGld_Cab.BlkGld_Cab"))
    (:`1`
      (`self.SetAccentMaterials` "/Game/Spkrs/m/WalSlv_Ft.WalSlv_Ft" "/Game/Spkrs/m/WalSlv_Cab.WalSlv_Cab"))
    (:`2`
      (`self.SetAccentMaterials` "/Game/Spkrs/m/TkBlk_Ft.TkBlk_Ft" "/Game/Spkrs/m/TkBlk_Cab.TkBlk_Cab"))
    (:`3`
      (`self.SetAccentMaterials` "/Game/Spkrs/m/EbStl_Ft.EbStl_Ft" "/Game/Spkrs/m/EbStl_Cab.EbStl_Cab"))
    (:`4`
      (`self.SetAccentMaterials` "/Game/Spkrs/m/WhtCp_Ft.WhtCp_Ft" "/Game/Spkrs/m/WhtCp_Cab.WhtCp_Cab")))
  (`self.DisplayAccentData` (`self.AccentIndex`)))

(fn `CabinetClicked`
  (bind _output_get (set `self.CabinetMaterialIndex` (mod (+ (`self.CabinetMaterialIndex`) 1) (`self.CabinetIndexMax`))))
  (switch `int` _output_get
    (:`0`
      (`self.SetCabinetMaterial` "/Game/Spkrs/m/BlkGld_Cab.BlkGld_Cab"))
    (:`1`
      (`self.SetCabinetMaterial` "/Game/Spkrs/m/WalSlv_Cab.WalSlv_Cab"))
    (:`2`
      (`self.SetCabinetMaterial` "/Game/Spkrs/m/TkBlk_Cab.TkBlk_Cab"))
    (:`3`
      (`self.SetCabinetMaterial` "/Game/Spkrs/m/EbStl_Cab.EbStl_Cab"))
    (:`4`
      (`self.SetCabinetMaterial` "/Game/Spkrs/m/WhtCp_Cab.WhtCp_Cab")))
  (`self.DisplayCabinetData` (`self.CabinetMaterialIndex`)))

(fn `DisplayAccentData`
  (params (Index :type Integer))
  (bind _returnvalue (`|GetDataTableRow` "/Game/Data/Accent_Data.Accent_Data" (`KismetStringLibrary.Conv_StringToName` (`KismetStringLibrary.Conv_IntToString` Index)))
    (:`then`
      (`|ExecutionSequence`
        (:`then_0`
          (bind (_shortdescription _longdescription _price) (break `/Game/Data/SpeakerDataStructure` _returnvalue))
          (set `self.Accent Short Description` _shortdescription))
        (:`then_1`
          (set `self.Accent Long Description` _longdescription))
        (:`then_2`
          (set `self.Accent Price` _price))
        (:`then_3`
          (`self.DisplayFinalDataToHUD`))))))

(fn `DisplayAccentHint`
  (locals (`Accent Hint Text` :type Text :default "NSLOCTEXT(\"\", \"C72E84314CCC5F13375AFE877DAD57FF\", \"Click to customize accents and feet\")"))
  (set `/Game/HUD/HUD_UI.ControllerHintText` (`local.Accent Hint Text`) (`self.HUD`)))

(fn `DisplayCabinetData`
  (params (Index :type Integer))
  (bind _returnvalue (`|GetDataTableRow` "/Game/Data/Cabinette_Data.Cabinette_Data" (`KismetStringLibrary.Conv_StringToName` (`KismetStringLibrary.Conv_IntToString` Index)))
    (:`then`
      (`|ExecutionSequence`
        (:`then_0`
          (bind (_shortdescription _longdescription _price) (break `/Game/Data/SpeakerDataStructure` _returnvalue))
          (set `self.Cabinet Short Description` _shortdescription))
        (:`then_1`
          (set `self.Cabinet Long Description` _longdescription))
        (:`then_2`
          (set `self.Cabinet Price` _price))
        (:`then_3`
          (`self.DisplayFinalDataToHUD`))))))

(fn `DisplayCabinetHint`
  (locals (`Cabinet Hint Text` :type Text :default "NSLOCTEXT(\"\", \"D285BE8D4362A059991CC4A9A8297D20\", \"Click to customize cabinet\")"))
  (set `/Game/HUD/HUD_UI.ControllerHintText` (`local.Cabinet Hint Text`) (`self.HUD`)))

(fn `DisplayFinalDataToHUD`
  (`|ExecutionSequence`
    (:`then_0`
      ;[1 1 1] Send Total Price To HUD
      (set `/Game/HUD/HUD_UI.TotalPrice` (`self.FormatPriceToString` (+ (`self.BasePrice`) (`self.Cabinet Price`) (`self.Speaker Price`) (`self.Accent Price`) (`self.Screen Price`))) (`self.HUD`)))
    (:`then_1`
      ;[1 1 1] Send Individual Prices To HUD
      (`|ExecutionSequence`
        (:`then_0`
          (set `/Game/HUD/HUD_UI.SpeakerPrice` (`self.FormatPriceToString` (`self.Speaker Price`)) (`self.HUD`)))
        (:`then_1`
          (set `/Game/HUD/HUD_UI.CabinetPrice` (`self.FormatPriceToString` (`self.Cabinet Price`)) (`self.HUD`)))
        (:`then_2`
          (set `/Game/HUD/HUD_UI.AccentPrice` (`self.FormatPriceToString` (`self.Accent Price`)) (`self.HUD`)))
        (:`then_3`
          (set `/Game/HUD/HUD_UI.ScreenPrice` (`self.FormatPriceToString` (`self.Screen Price`)) (`self.HUD`)))
        (:`then_4`
          (set `/Game/HUD/HUD_UI.BasePrice` (`self.FormatPriceToString` (`self.BasePrice`)) (`self.HUD`)))))
    (:`then_2`
      ;[1 1 1] Send Choices to HUD
      (set `/Game/HUD/HUD_UI.ScreenChoice` (`self.Screen Short Description`) (`self.HUD`))
      (set `/Game/HUD/HUD_UI.CabinetChoice` (`self.Cabinet Short Description`) (`self.HUD`))
      (set `/Game/HUD/HUD_UI.AccentChoice` (`self.Accent Short Description`) (`self.HUD`))
      (set `/Game/HUD/HUD_UI.SpeakerChoice` (`self.Speaker Short Description`) (`self.HUD`)))
    (:`then_3`
      ;[1 1 1] Send Description to HUD
      (set `/Game/HUD/HUD_UI.Long Description` (`KismetTextLibrary.Conv_StringToText` (`KismetStringLibrary.Concat_StrStr` (`KismetTextLibrary.Conv_TextToString` (`self.Speaker Long Description`)) " mounted in " (`KismetTextLibrary.Conv_TextToString` (`self.Cabinet Long Description`)) " cabinets and " (`KismetTextLibrary.Conv_TextToString` (`self.Accent Long Description`)) " trim")) (`self.HUD`)))))

(fn `DisplayGeneralHint`
  (locals (`General hint text` :type Text :default "NSLOCTEXT(\"\", \"62B963C9484B3C72CD59A498880B182B\", \"Click on any component to customize\")"))
  (set `/Game/HUD/HUD_UI.ControllerHintText` (`local.General hint text`) (`self.HUD`)))

(fn `DisplayScreenData`
  (params (Index :type Integer))
  (bind _returnvalue (`|GetDataTableRow` "/Game/Data/Screen_Data.Screen_Data" (`KismetStringLibrary.Conv_StringToName` (`KismetStringLibrary.Conv_IntToString` Index)))
    (:`then`
      (`|ExecutionSequence`
        (:`then_0`
          (bind (_shortdescription _longdescription _price) (break `/Game/Data/SpeakerDataStructure` _returnvalue))
          (set `self.Screen Short Description` _shortdescription))
        (:`then_1`
          (set `self.Screen Long Description` _longdescription))
        (:`then_2`
          (set `self.Screen Price` _price))
        (:`then_3`
          (`self.DisplayFinalDataToHUD`))))))

(fn `DisplayScreenHint`
  (locals (`Screen Hint Text` :type Text :default "NSLOCTEXT(\"\", \"709A96EC40565BC31BA4B9928BB584AB\", \"Click to customize speaker screen mesh\")"))
  (set `/Game/HUD/HUD_UI.ControllerHintText` (`local.Screen Hint Text`) (`self.HUD`)))

(fn `DisplaySpeakerData`
  (params (Index :type Integer))
  (bind _returnvalue (`|GetDataTableRow` "/Game/Data/Speaker_Data.Speaker_Data" (`KismetStringLibrary.Conv_StringToName` (`KismetStringLibrary.Conv_IntToString` Index)))
    (:`then`
      (`|ExecutionSequence`
        (:`then_0`
          (bind (_shortdescription _longdescription _price) (break `/Game/Data/SpeakerDataStructure` _returnvalue))
          (set `self.Speaker Short Description` _shortdescription))
        (:`then_1`
          (set `self.Speaker Long Description` _longdescription))
        (:`then_2`
          (set `self.Speaker Price` _price))
        (:`then_3`
          (`self.DisplayFinalDataToHUD`))))))

(fn `DisplaySpeakerHint`
  (locals (`Speaker hint text` :type Text :default "NSLOCTEXT(\"\", \"E27336D64A1FDB075DF97099630F5B28\", \"Click to customise speakers and tweeters\")"))
  (set `/Game/HUD/HUD_UI.ControllerHintText` (`local.Speaker hint text`) (`self.HUD`)))

(fn `FormatPriceToString`
  (params (Price :type Integer))
  (returns (FormattedPrice :type Text))
  (return (`KismetTextLibrary.AsCurrencyBase` Price "GBP")))

(fn `InitialiseSpeakerController`
  (params (SpeakerComponents :type "Array of /Game/Spkrs/BP/Speaker_BP Object Reference") (HUD :type "/Game/HUD/HUD_UI Object Reference"))
  (`|ExecutionSequence`
    (:`then_0`
      ;[1 1 1] Reference to Speakers in Scene
      (set `self.SpeakerList` SpeakerComponents))
    (:`then_1`
      ;[1 1 1] Reference to HUD
      (set `self.HUD` HUD))
    (:`then_2`
      ;[1 1 1] Update HUD With Initial Data
      (`self.DisplayCabinetData` 0)
      (`self.DisplayAccentData` 0)
      (`self.DisplayScreenData` 0)
      (`self.DisplaySpeakerData` 0))))

(fn `PlayAudio`
  (params (TrackIndex :type Integer))
  (bind _music_player (`self.Music Player`))
  (`|ExecutionSequence`
    (:`then_0`
      ;[1 1 1] Stop Playing Audio
      (`AudioComponent.Stop` (`self.Music Player`)))
    (:`then_1`
      ;[1 1 1] Load Audio Track
      (`AudioComponent.SetSound` (`self.Music Player`) (`|GetArrayItem` (`self.MusicTracks`) TrackIndex)))
    (:`then_2`
      ;[1 1 1] Play Audio
      (`AudioComponent.Play` _music_player 0.0)
      (`AudioComponent.AdjustVolume` _music_player 0.0 (`self.MusicVolume`) "Linear"))))

(fn `ScreenClicked`
  (bind _output_get (set `self.ScreenIndex` (mod (+ (`self.ScreenIndex`) 1) (`self.ScreenIndexMax`))))
  (switch `int` _output_get
    (:`0`
      ;[1 1 1] Black
      (`self.SetScreenColour` (0.0 0.0 0.0)))
    (:`1`
      ;[1 1 1] Gold
      (`self.SetScreenColour` (0.1441 0.1155 0.0323)))
    (:`2`
      ;[1 1 1] Dark Gray
      (`self.SetScreenColour` (0.089 0.089 0.089)))
    (:`3`
      ;[1 1 1] White
      (`self.SetScreenColour` (1.0 1.0 1.0)))
    (:`4`
      ;[1 1 1] Dark Brown
      (`self.SetScreenColour` (0.642 0.237 0.0093))))
  (`self.DisplayScreenData` (`self.ScreenIndex`)))

(fn `SetAccentMaterials`
  (params (FootMaterial :type "Material Object Reference") (AccentMaterial :type "Material Object Reference"))
  (for _array_element (`self.SpeakerList`)
    (bind (_footmeshes _accentmeshes) (`/Game/Spkrs/BP/Speaker_BP.GetAccentComponents` _array_element))
    (`|ExecutionSequence`
      (:`then_0`
        (for _array_element_2 _footmeshes
          (`PrimitiveComponent.SetMaterial` _array_element_2 0 FootMaterial)))
      (:`then_1`
        (for _array_element_3 _accentmeshes
          (`PrimitiveComponent.SetMaterial` _array_element_3 0 AccentMaterial))))))

(fn `SetBackgroundColour`
  (params (ColourToSet :type "Vector Structure"))
  (`MeshComponent.SetVectorParameterValueOnMaterials` (`self.RoomMeshRef`) "BaseColour" ColourToSet))

(fn `SetCabinetMaterial`
  (params (OurMaterial :type "Material Object Reference"))
  (for _array_element (`self.SpeakerList`)
    (bind _cabinetmesh (`/Game/Spkrs/BP/Speaker_BP.GetCabinetComponent` _array_element))
    (`PrimitiveComponent.SetMaterial` _cabinetmesh 0 OurMaterial)))

(fn `SetScreenColour`
  (params (Colour :type "Vector Structure"))
  (for _array_element (`self.SpeakerList`)
    (bind _screenmesh (`/Game/Spkrs/BP/Speaker_BP.GetScreenComponent` _array_element))
    (`MeshComponent.SetVectorParameterValueOnMaterials` _screenmesh "Color" Colour)))

(fn `SetSpeakerMaterials`
  (params (TweeterMaterial :type "Material Object Reference") (SpeakerMaterial :type "Material Object Reference"))
  (for _array_element (`self.SpeakerList`)
    (bind (_tweetermesh _speakermesh) (`/Game/Spkrs/BP/Speaker_BP.GetSpeakerComponents` _array_element))
    (`|ExecutionSequence`
      (:`then_0`
        (`PrimitiveComponent.SetMaterial` _tweetermesh 0 TweeterMaterial))
      (:`then_1`
        (`PrimitiveComponent.SetMaterial` _speakermesh 0 SpeakerMaterial)))))

(fn `SpeakerClicked`
  (bind _output_get (set `self.SpeakerMaterialIndex` (mod (+ (`self.SpeakerMaterialIndex`) 1) (`self.SpeakerIndexMax`))))
  (switch `int` _output_get
    (:`0`
      (`self.SetSpeakerMaterials` "/Game/Spkrs/m/BlkGld_Twt.BlkGld_Twt" "/Game/Spkrs/m/BlkGld_Wof.BlkGld_Wof"))
    (:`1`
      (`self.SetSpeakerMaterials` "/Game/Spkrs/m/WalSlv_Twt.WalSlv_Twt" "/Game/Spkrs/m/WalSlv_Wof.WalSlv_Wof"))
    (:`2`
      (`self.SetSpeakerMaterials` "/Game/Spkrs/m/TkBlk_Twt.TkBlk_Twt" "/Game/Spkrs/m/TkBlk_Wof.TkBlk_Wof"))
    (:`3`
      (`self.SetSpeakerMaterials` "/Game/Spkrs/m/WhtCp_Twt.WhtCp_Twt" "/Game/Spkrs/m/WhtCp_Wof.WhtCp_Wof")))
  (`self.DisplaySpeakerData` (`self.SpeakerMaterialIndex`)))

(fn `UpdateMusicVolume`
  (params (NewVolume :type "Float (double-precision)"))
  (bind _output_get (set `self.MusicVolume` NewVolume))
  (`AudioComponent.AdjustVolume` (`self.Music Player`) 0.0 _output_get "Linear"))

(fn `UserConstructionScript`)